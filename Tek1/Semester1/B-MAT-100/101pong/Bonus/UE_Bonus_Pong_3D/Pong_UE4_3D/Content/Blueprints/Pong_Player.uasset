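; Player paddle for a Pong game, which also creates the Score widget and adds it to the viewport on BeginPlay.
; Each Tick, it offsets its Cube along local X by scaled axis input, clamped between SpeedMin and SpeedMax, without delta-time scaling.
; ChangingSpeed sets both limits, so the allowed movement range can be changed at runtime.
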(event `self.ReceiveBeginPlay`
  (bind _returnvalue (`|CreateWidget` "/Game/Blueprints/Score.Score_C"))
  (`UserWidget.AddToViewport` _returnvalue 0))

(event `self.ReceiveTick`
  (params (DeltaSeconds :type "Float (single-precision)"))
  (`SceneComponent.K2_AddLocalOffset` (`self.Cube`) (`KismetMathLibrary.MakeVector` (`KismetMathLibrary.FClamp` (* (`self.GetInputAxisKeyValue`) 10.0) (`self.Speed_Min`) (`self.Speed_Max`))) false false))

(fn `Changing_Speed`
  (params (Speed_Min :type "Float (double-precision)") (Speed_Max :type "Float (double-precision)"))
  (set `self.Speed_Min` Speed_Min)
  (set `self.Speed_Max` Speed_Max))

(fn `UserConstructionScript`)