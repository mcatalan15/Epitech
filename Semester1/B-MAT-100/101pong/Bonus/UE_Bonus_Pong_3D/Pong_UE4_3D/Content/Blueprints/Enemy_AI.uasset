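; Enemy AI Blueprint that slides its Cube sideways to follow the Ball, like an opposing paddle.
; On each Tick, throttled by TickInterval, it looks up the Ball actor and stores its Sphere's relative location.
; Move then runs MoveComponentTo over TimeMoving toward the ball's X, clamped to fixed bounds, with Y and Z held constant.
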(event `self.ReceiveBeginPlay`
  (`self.SetActorTickInterval` (`self.Tick Interval`)))

(event `self.ReceiveTick`
  (params (DeltaSeconds :type "Float (single-precision)"))
  (bind _returnvalue (`GameplayStatics.GetActorOfClass` "/Game/Blueprints/Ball.Ball_C"))
  (`/Engine/EditorBlueprintResources/StandardMacros.IsValid` _returnvalue
    (:`Is Valid`
      (set `self.Ball_Loc` (`SceneComponent.RelativeLocation` (`/Game/Blueprints/Ball.Sphere` _returnvalue)))
      (`self.Move`))))

(event `Move`
  (bind _ball_loc_x (`KismetMathLibrary.BreakVector` (`self.Ball_Loc`)))
  (`KismetSystemLibrary.MoveComponentTo` (`self.Cube`) (`KismetMathLibrary.MakeVector` (`KismetMathLibrary.FClamp` _ball_loc_x -450.0 390.0) 650.0 150.0) (struct) false false (`self.Time_Moving`)))

(fn `UserConstructionScript`)